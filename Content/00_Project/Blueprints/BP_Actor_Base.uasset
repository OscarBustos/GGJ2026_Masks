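; Base actor Blueprint for objects that appear only while the current mask matches their RequiredMask.
; OnMaskChanged hides the actor on a mismatch and shows it on a match if it is not already visible.
; Show and HIde toggle in-game visibility and the static mesh's collision together, tracking the state in IsVisible.
; Hiding runs on every mismatch, as the IsVisible check for that branch is left unconnected.
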(event `/Game/00_Project/Blueprints/Interfaces/BPI_MaskReact.OnMaskChanged`
  (params (CurrentMask :type "/Game/00_Project/Enums/E_Mask Enum" :default "NewEnumerator0"))
  (if (`|EnumInequality` CurrentMask (`self.RequiredMask`))
    (`self.HIde`)
    (elif (and (`|EnumEquality` CurrentMask (`self.RequiredMask`)) (not (`self.isVisible`)))
      (`self.Show`))))

(fn `HIde`
  (`self.SetActorHiddenInGame` self true)
  (`PrimitiveComponent.SetCollisionEnabled` (`self.StaticMesh`) "NoCollision")
  (set `self.isVisible` false))

(fn `Show`
  (`self.SetActorHiddenInGame` self false)
  (`PrimitiveComponent.SetCollisionEnabled` (`self.StaticMesh`) "QueryAndPhysics")
  (set `self.isVisible` true))

(fn `UserConstructionScript`)