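; Player character that collects and wears five masks: Demon, Wolf, Gas, Welding and Knocker.
; Overlapping a tagged BP_Collectable stores it, and Collect unlocks its mask type and destroys it.
; OnMaskChange hides all mask meshes, shows the requested one if unlocked, and broadcasts OnMaskChanged, falling back to None if locked.
; Each change triggers forward and reverse timelines on FollowCamera's post-process blend weight, whose settings can be replaced through UpdatePostProcessSettings.
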(event `self.ReceiveBeginPlay`
  (set `self.MapMasks` (`|MakeArray` (`self.WeldingMask`) (`self.KnockerMask`) (`self.GasMask`) (`self.DemonMask`) (`self.WolfMask`))))

(event `PlayTransition`
  (params (Reverse :type Boolean))
  (if Reverse
    (bind (_direction _blend) (`Timeline|Timeline_0` :!via `ReverseFromEnd`)
      (:`Update`
        (`CameraComponent.SetPostProcessBlendWeight` (`self.FollowCamera`) _blend)))
    (else
      (bind (_direction_2 _blend_2) (`Timeline|Timeline`)
        (:`Update`
          (`CameraComponent.SetPostProcessBlendWeight` (`self.FollowCamera`) _blend_2))))))

(event `self.ReceiveActorBeginOverlap`
  (params (OtherActor :type "Actor Object Reference"))
  (`/Engine/EditorBlueprintResources/StandardMacros.IsValid` OtherActor
    (:`Is Valid`
      (if (`self.ActorHasTag` OtherActor "Collect")
        (bind _asbp_collectable (cast `/Game/00_Project/Blueprints/BP_Collectable` OtherActor))
        (set `self.CurrentCollectible` _asbp_collectable)))))

(event `self.ReceiveActorEndOverlap`
  (params (OtherActor :type "Actor Object Reference"))
  (`/Engine/EditorBlueprintResources/StandardMacros.IsValid` OtherActor
    (:`Is Valid`
      (if (`self.ActorHasTag` "Collect")
        (cast `/Game/00_Project/Blueprints/Interfaces/BPI_Collectible` OtherActor)
        (set `self.CurrentCollectible` null)))))

(fn `Collect`
  (`/Engine/EditorBlueprintResources/StandardMacros.IsValid` (`self.CurrentCollectible`)
    (:`Is Valid`
      (bind _type (`/Game/00_Project/Blueprints/Interfaces/BPI_Collectible.getType` (`self.CurrentCollectible`)))
      (switch `/Game/00_Project/Enums/E_Collectible_Type` _type
        (:`NewEnumerator0`
          (bind _mask (`/Game/00_Project/Blueprints/Interfaces/BPI_Collectible.getMask` (`self.CurrentCollectible`)))
          (switch `/Game/00_Project/Enums/E_Mask` _mask
            (:`NewEnumerator0`
              _)
            (:`NewEnumerator1`
              (set `self.DemonMaskEnabled` true))
            (:`NewEnumerator2`
              (set `self.WolfMaskEnabled` true))
            (:`NewEnumerator3`
              (set `self.GasMaskEnable` true))
            (:`NewEnumerator4`
              (set `self.WeldingMaskEnable` true))
            (:`NewEnumerator5`
              (set `self.KnockerMaskEnable` true)))
          (`self.K2_DestroyActor` (`self.CurrentCollectible`))
          (set `self.CurrentCollectible` null))))))

(fn `EnableMask`
  (params (Enabled :type Boolean) (Mask :type "/Game/00_Project/Enums/E_Mask Enum" :default "NewEnumerator0") (Mesh :type "StaticMeshComponent Object Reference"))
  (if Enabled
    (`self.PlayTransition` false)
    (`self.OnMaskChanged` Mask)
    (`/Engine/EditorBlueprintResources/StandardMacros.IsValid` Mesh
      (:`Is Valid`
        (`SceneComponent.SetHiddenInGame` Mesh (not (`local.Enabled`)) false))
      (:`Is Not Valid`
        _))
    (`self.PlayTransition` true)
    (else
      (`self.PlayTransition` false)
      (`self.OnMaskChanged` "NewEnumerator0")
      (`self.PlayTransition` true))))

(fn `IsMaskEnabled`
  (params (Mask :type "/Game/00_Project/Enums/E_Mask Enum" :default "NewEnumerator0"))
  (returns (Enabled :type Boolean))
  (switch `/Game/00_Project/Enums/E_Mask` Mask
    (:`NewEnumerator0`
      (return true))
    (:`NewEnumerator1`
      (return (`self.DemonMaskEnabled`)))
    (:`NewEnumerator2`
      (return (`self.WolfMaskEnabled`)))
    (:`NewEnumerator3`
      (return (`self.GasMaskEnable`)))
    (:`NewEnumerator4`
      (return (`self.WeldingMaskEnable`)))
    (:`NewEnumerator5`
      (return (`self.KnockerMaskEnable`)))))

(fn `OnMaskChange`
  (params (Mask :type "/Game/00_Project/Enums/E_Mask Enum" :default "NewEnumerator0"))
  (for _array_element (`self.MapMasks`)
    (`SceneComponent.SetHiddenInGame` _array_element true false))
  (switch `/Game/00_Project/Enums/E_Mask` Mask
    (:`NewEnumerator0`
      (`self.EnableMask` false))
    (:`NewEnumerator1`
      (`self.EnableMask` (`self.DemonMaskEnabled`) (`local.Mask`) (`self.DemonMask`)))
    (:`NewEnumerator2`
      (`self.EnableMask` (`self.WolfMaskEnabled`) (`local.Mask`) (`self.WolfMask`)))
    (:`NewEnumerator3`
      (`self.EnableMask` (`self.GasMaskEnable`) (`local.Mask`) (`self.GasMask`)))
    (:`NewEnumerator4`
      (`self.EnableMask` (`self.WeldingMaskEnable`) (`local.Mask`) (`self.WeldingMask`)))
    (:`NewEnumerator5`
      (`self.EnableMask` (`self.KnockerMaskEnable`) (`local.Mask`) (`self.KnockerMask`)))))

(fn `UpdatePostProcessSettings`
  (params (Settings :type "PostProcessSettings Structure"))
  (set `CameraComponent.PostProcessSettings` Settings (`self.FollowCamera`)))

(fn `UserConstructionScript`
  (`parent.UserConstructionScript`))