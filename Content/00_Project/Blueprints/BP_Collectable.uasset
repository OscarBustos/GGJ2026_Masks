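; BP_Collectable is a collectable actor that shows a widget while the player's BP_Character is near it.
; Box overlap reveals the widget and actor end-overlap hides it, with an IsVisible flag guarding both changes.
; While visible, Tick rotates the widget to face the camera manager cached at BeginPlay.
; GetMask and GetType expose the Mask and ObjectType variables; the file contains no pickup logic.
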(event `self.ReceiveBeginPlay`
  (bind _asbp_character (cast `/Game/00_Project/Blueprints/BP_Character` (`GameplayStatics.GetPlayerPawn` 0)))
  (set `self.BP Character` _asbp_character)
  (set `self.CameraManager` (`GameplayStatics.GetPlayerCameraManager` 0)))

(event `self.ReceiveTick`
  (params (DeltaSeconds :type "Float (single-precision)"))
  (bind _widget (`self.Widget`))
  (if (`self.isVisible`)
    (`SceneComponent.K2_SetWorldRotation` _widget (`KismetMathLibrary.FindLookAtRotation` (`SceneComponent.K2_GetComponentLocation` _widget) (`PlayerCameraManager.GetCameraLocation` (`self.CameraManager`))) false false)))

(event `self.Box.OnComponentBeginOverlap`
  (params (OverlappedComponent :type "PrimitiveComponent Object Reference") (OtherActor :type "Actor Object Reference") (OtherComp :type "PrimitiveComponent Object Reference") (OtherBodyIndex :type Integer) (bFromSweep :type Boolean) (SweepResult :type "HitResult Structure (by ref)"))
  (if (and (== OtherActor (`self.BP Character`)) (not (`self.isVisible`)))
    (`SceneComponent.SetHiddenInGame` (`self.Widget`) false false)
    (set `self.isVisible` true)))

(event `self.ReceiveActorEndOverlap`
  (params (OtherActor :type "Actor Object Reference"))
  (if (and (== OtherActor (`self.BP Character`)) (`self.isVisible`))
    (`SceneComponent.SetHiddenInGame` (`self.Widget`) true false)
    (set `self.isVisible` false)))

(event `getMask_1_1`)

(fn `getMask`
  (returns (Mask :type "/Game/00_Project/Enums/E_Mask Enum"))
  (return (`self.Mask`)))

(fn `getType`
  (returns (Type :type "/Game/00_Project/Enums/E_Collectible_Type Enum"))
  (return (`self.ObjectType`)))

(fn `UserConstructionScript`)