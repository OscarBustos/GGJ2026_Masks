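; Trap actor with swinging blades that responds to the player collecting a specific mask.
; On BeginPlay it binds to the character's mask-collected event and caches the blades child actor; the matching mask sets Collected and calls Show.
; If not yet Enabled, Show enables the trap, runs parent Show, activates the blades, then hides them.
; Once collected, the overridden Show and HIde toggle blade mesh visibility.
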(event `self.ReceiveBeginPlay`
  (`parent.ReceiveBeginPlay`)
  (bind _asbp_character (cast `/Game/00_Project/Blueprints/BP_Character` (`GameplayStatics.GetPlayerCharacter` 0)))
  (add `/Game/00_Project/Blueprints/BP_Character.OnMaskCollected` _asbp_character (delegate `OnMaskCollected`))
  (bind _asbp_swinging_blades (cast `/Game/AssortmentOfTraps/Traps/BluePrints/1_SwingingBlades/BP_SwingingBlades` (`ChildActorComponent.ChildActor` (`self.BP_SwingingBlades`))))
  (set `self.BP Swinging Blades` _asbp_swinging_blades))

(event `OnMaskCollected`
  (params (Mask :type "/Game/00_Project/Enums/E_Mask Enum" :default "NewEnumerator0"))
  (if (and (`|EnumEquality` Mask "NewEnumerator1") (not (`self.Collected`)))
    (set `self.Collected` true)
    (`self.Show`)))

(fn `HIde`
  (if (`self.Collected`)
    (set `self.isVisible` false)
    (`/Game/AssortmentOfTraps/Traps/BluePrints/1_SwingingBlades/BP_SwingingBlades.HideMesh` (`self.BP Swinging Blades`))
    (else
      (`parent.HIde`))))

(fn `NewFunction`)

(fn `Show`
  (if (`self.Collected`)
    (if (`self.Enabled`)
      (set `self.isVisible` true)
      (`/Game/AssortmentOfTraps/Traps/BluePrints/1_SwingingBlades/BP_SwingingBlades.ShowMesh` (`self.BP Swinging Blades`))
      (else
        (set `self.Enabled` true)
        (`parent.Show`)
        (`/Game/AssortmentOfTraps/Traps/BluePrints/1_SwingingBlades/BP_SwingingBlades.Activate` (`self.BP Swinging Blades`))
        (`self.HIde`)))))

(fn `UserConstructionScript`
  (`parent.UserConstructionScript`))