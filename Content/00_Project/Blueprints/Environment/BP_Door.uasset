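; Door actor whose collision is switched on and off through actions inherited from its parent class.
; It turns actor collision off at BeginPlay, so it starts without collision.
; The EnableActions and DisableActions overrides call the parent versions, then turn collision on and off respectively.
; Tick is disabled, and the overlap event and construction script add no logic of their own.
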(event `self.ReceiveBeginPlay`
  (`parent.ReceiveBeginPlay`)
  (`self.SetActorEnableCollision` false))

(event `self.ReceiveActorBeginOverlap`
  (params (OtherActor :type "Actor Object Reference")))

(fn `DisableActions`
  (`parent.DisableActions`)
  (`self.SetActorEnableCollision` false))

(fn `EnableActions`
  (`parent.EnableActions`)
  (`self.SetActorEnableCollision` true))

(fn `UserConstructionScript`
  (`parent.UserConstructionScript`))