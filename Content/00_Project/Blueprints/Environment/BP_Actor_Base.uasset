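; Base environment actor that appears or disappears according to the player's active mask.
; BeginPlay caches the player's BP_Character, which OnMaskChanged queries to check that DisplayMask is enabled.
; A matching enabled mask toggles visibility; otherwise the actor reverts to the default implied by HideWhenMask.
; Show and HIde switch rendering and mesh collision, then call the empty EnableActions and DisableActions hooks.
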(event `self.ReceiveBeginPlay`
  (bind _asbp_character (cast `/Game/00_Project/Blueprints/BP_Character` (`GameplayStatics.GetPlayerPawn` 0)))
  (set `self.BP Character` _asbp_character))

(event `/Game/00_Project/Blueprints/Interfaces/BPI_MaskReact.OnMaskChanged`
  (params (CurrentMask :type "/Game/00_Project/Enums/E_Mask Enum" :default "NewEnumerator0"))
  (bind _enabled (`/Game/00_Project/Blueprints/BP_Character.IsMaskEnabled` (`self.BP Character`) (`self.DisplayMask`)))
  (if (and _enabled (`|EnumEquality` CurrentMask (`self.DisplayMask`)))
    (if (and (`self.HideWhenMask`) (`self.isVisible`))
      (`self.HIde`)
      (elif (and (`self.HideWhenMask`) (not (`self.isVisible`)))
        (`self.Show`)
        (elif (and (not (`self.HideWhenMask`)) (not (`self.isVisible`)))
          (`self.Show`)
          (elif (and (not (`self.HideWhenMask`)) (`self.isVisible`))
            (`self.HIde`)))))
    (elif (and (`self.HideWhenMask`) (`self.isVisible`))
      _
      (elif (and (`self.HideWhenMask`) (not (`self.isVisible`)))
        (`self.Show`)
        (elif (and (not (`self.HideWhenMask`)) (not (`self.isVisible`)))
          _
          (elif (and (not (`self.HideWhenMask`)) (`self.isVisible`))
            (`self.HIde`)))))))

(fn `DisableActions`
  (return))

(fn `EnableActions`
  (return))

(fn `HIde`
  (`self.SetActorHiddenInGame` self true)
  (`PrimitiveComponent.SetCollisionEnabled` (`self.StaticMesh`) "NoCollision")
  (set `self.isVisible` false)
  (`self.DisableActions`))

(fn `Show`
  (`self.SetActorHiddenInGame` self false)
  (`PrimitiveComponent.SetCollisionEnabled` (`self.StaticMesh`) "QueryAndPhysics")
  (set `self.isVisible` true)
  (`self.EnableActions`))

(fn `UserConstructionScript`)