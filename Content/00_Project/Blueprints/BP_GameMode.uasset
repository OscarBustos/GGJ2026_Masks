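; Game mode that runs the menu, play and game-over flow and owns the UI widgets.
; On begin play it binds the player character's hurt and game-over events, creates the game-over, main menu and life bar widgets, then pauses behind the menu.
; Play removes the menu, unpauses and shows the life bar, which updates on each hit.
; Game over pauses again and shows the game-over screen with the mouse cursor.
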(event `self.ReceiveBeginPlay`
  (bind _returnvalue (`GameplayStatics.GetPlayerController` 0))
  (bind _asbp_character (cast `/Game/00_Project/Blueprints/BP_Character` (`GameplayStatics.GetPlayerCharacter` 0)))
  (bind _output_get (set `self.BP Character` _asbp_character))
  (add `/Game/00_Project/Blueprints/BP_Character.OnGameOver` _output_get (delegate `OnGameOver`))
  (add `/Game/00_Project/Blueprints/BP_Character.OnHurt` _output_get (delegate `OnHurt`))
  (bind _returnvalue_2 (`|CreateWidget` "/Game/00_Project/Blueprints/Widgets/WBP_GameOver.WBP_GameOver_C"))
  (set `self.WBP_GameOver` _returnvalue_2)
  (bind _returnvalue_3 (`|CreateWidget` "/Game/00_Project/Blueprints/Widgets/WBP_MainMenu.WBP_MainMenu_C"))
  (bind _output_get_2 (set `self.WBP_MainMenu` _returnvalue_3))
  (`UserWidget.AddToViewport` _output_get_2 0)
  (set `PlayerController.bShowMouseCursor` true _returnvalue)
  (`WidgetBlueprintLibrary.SetInputMode_GameAndUIEx` _returnvalue null "DoNotLock" false)
  (`GameplayStatics.SetGamePaused` true)
  (bind _returnvalue_4 (`|CreateWidget` "/Game/00_Project/Blueprints/Widgets/WBP_LiveBar.WBP_LiveBar_C"))
  (set `self.Bar` _returnvalue_4))

(event `OnHurt`
  (params (Damge :type "Float (double-precision)"))
  (`/Game/00_Project/Blueprints/Widgets/WBP_LiveBar.HandleDamage` (`self.Bar`) Damge (`KismetMathLibrary.Conv_IntToDouble` (`/Game/00_Project/Blueprints/BP_Character.MaxLive` (stale `self.ReceiveBeginPlay` _output_get)))))

(event `OnGameOver`
  (bind _returnvalue (`GameplayStatics.GetPlayerController` 0))
  (bind _wbp_gameover (`self.WBP_GameOver`))
  (`GameplayStatics.SetGamePaused` true)
  (`UserWidget.AddToViewport` _wbp_gameover 0)
  (set `PlayerController.bShowMouseCursor` true _returnvalue)
  (`WidgetBlueprintLibrary.SetInputMode_GameAndUIEx` _returnvalue _wbp_gameover "DoNotLock" false))

(event `Play`
  (bind _returnvalue (`GameplayStatics.GetPlayerController` 0))
  (`Widget.RemoveFromParent` (`self.WBP_MainMenu`))
  (`WidgetBlueprintLibrary.SetInputMode_GameOnly` _returnvalue)
  (set `PlayerController.bShowMouseCursor` false _returnvalue)
  (`GameplayStatics.SetGamePaused` false)
  (`UserWidget.AddToViewport` (`self.Bar`) 0))

(fn `UserConstructionScript`)